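; A grabbable hand mirror prop that carries a working mirror with left and right eye scene captures.
; On BeginPlay it snaps the mirror to an attach point, hides itself from both captures, and gives the mirror surface a collisionless disc mesh scaled like the preview mesh.
; Both grab components simulate physics on drop and trigger a check that, if enabled, stops physics and moves the prop to a stored transform.
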(event Custom|CheckTeleport
  (if (Variables|Default|GetbShouldTeleport)
    (Physics|SetSimulatePhysics (Variables|Default|GetStaticMesh) false)
    (Transformation|SetActorTransform (Variables|Default|GetTeleportTransform))))

(event EventBeginPlay
  (bind _self self)
  (bind _attachedmirror (Variables|Default|GetAttachedMirror))
  (bind _mirrormesh (Variables|/Script/UE5_Mirrors.CVrMirror|GetMirrorMesh _attachedmirror))
  (Variables|/Game/VRTemplate/Blueprints/GrabComponent.GrabComponent_C|SetbSimulateOnDrop (Variables|Default|GetGrabComponentSnap) true)
  (Variables|/Game/VRTemplate/Blueprints/GrabComponent.GrabComponent_C|SetbSimulateOnDrop (Variables|Default|GetGrabComponent) true)
  (EventDispatchers|BindEventtoOnDropped (Variables|Default|GetGrabComponent) (delegate Custom|CheckTeleport))
  (EventDispatchers|BindEventtoOnDropped (Variables|Default|GetGrabComponentSnap) (delegate Custom|CheckTeleport))
  (Transformation|AttachComponentToComponent _attachedmirror (Variables|Default|GetMirrorAttachPoint) "None" "SnapToTarget" "SnapToTarget" "SnapToTarget" false)
  (Utilities|Array|AddUnique (Variables|/Script/Engine.SceneCaptureComponent|GetHiddenActors (Variables|/Script/UE5_Mirrors.CVrMirror|GetSceneCaptureLeftEye _attachedmirror)) _self)
  (Utilities|Array|AddUnique (Variables|/Script/Engine.SceneCaptureComponent|GetHiddenActors (Variables|/Script/UE5_Mirrors.CVrMirror|GetSceneCaptureRightEye _attachedmirror)) _self)
  (Collision|SetCollisionEnabled _mirrormesh "NoCollision")
  (Transformation|SetRelativeScale3D _mirrormesh (Variables|/Script/Engine.SceneComponent|GetRelativeScale3D (Variables|Default|GetPreviewMesh)))
  (Components|StaticMesh|SetStaticMesh _mirrormesh "/Game/Mirrors/Meshes/SM_Mirror_Disc_1_Unit.SM_Mirror_Disc_1_Unit"))

(fn ConstructionScript)